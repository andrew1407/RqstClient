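; BP_StrategyActivator is a trigger actor that assigns a connection strategy to any RqstClientCharacter entering its box.
; BeginPlay lets command-line host and port arguments override the defaults, then registers them as options for its strategy type.
; On overlap, it passes the type, host, port and character to ConnectionStrategy.
; The construction script titles it with the resulting type://host:port endpoint from defaults, while setter events style the title and effect color.
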(event `self.ReceiveBeginPlay`
  (bind _returnvalue (`ClientFormUtils.GetPortCmdArgument`))
  (bind _returnvalue_2 (`ClientFormUtils.GetHostCmdArgument`))
  ;[1 0.2837 0] Set client options (command line or defaults input)
  (`parent.ReceiveBeginPlay`)
  (`|ExecutionSequence`
    (:`then_0`
      (if (not (`KismetStringLibrary.IsEmpty` _returnvalue_2))
        (set `self.Host` _returnvalue_2)))
    (:`then_1`
      (if (> _returnvalue 0)
        (set `self.Port` _returnvalue)))
    (:`then_2`
      (`ConnectionStrategyComponent.SetStrategyOptions` (`self.ConnectionStrategy`) (`self.StrategyType`) (`self.Host`) (`self.Port`)))))

(event `self.SetTitleText`
  (params (Text :type "Text (by ref)"))
  ;[0 0.1212 1] Strategy Activator methods implementation
  (`TextRenderComponent.K2_SetText` (`self.StrategyTitle`) Text))

(event `self.SetTitleColor`
  (params (Color :type "LinearColor Structure (by ref)"))
  ;[0 0.1212 1] Strategy Activator methods implementation
  (`TextRenderComponent.SetTextRenderColor` (`self.StrategyTitle`) (`KismetMathLibrary.Conv_LinearColorToColor` Color)))

(event `self.SetShiningColor`
  (params (Color :type "LinearColor Structure (by ref)"))
  ;[0 0.1212 1] Strategy Activator methods implementation
  (bind _output_get (set `self.color` Color))
  (`FXSystemComponent.SetVectorParameter` (`self.fx`) "Color" (`KismetMathLibrary.Conv_LinearColorToVector` _output_get)))

(event `self.Box.OnComponentBeginOverlap`
  (params (OverlappedComponent :type "PrimitiveComponent Object Reference") (OtherActor :type "Actor Object Reference") (OtherComp :type "PrimitiveComponent Object Reference") (OtherBodyIndex :type Integer) (bFromSweep :type Boolean) (SweepResult :type "HitResult Structure (by ref)"))
  (bind _asrqst_client_character (cast `RqstClientCharacter` OtherActor))
  (`ConnectionStrategyComponent.SetStrateryClient` (`self.ConnectionStrategy`) (`self.StrategyType`) (`self.Host`) (`self.Port`) _asrqst_client_character))

(fn `UserConstructionScript`
  (bind _strategytype (`self.StrategyType`))
  (bind _returnvalue (`|GetEnumeratorNameAsString` _strategytype))
  (`parent.UserConstructionScript`)
  (if (`|EnumEquality` _strategytype "NONE")
    (`StrategyActivator.SetTitleText` (`KismetTextLibrary.Conv_StringToText` _returnvalue))
    (else
      (`StrategyActivator.SetTitleText` (`KismetTextLibrary.Conv_StringToText` (`KismetStringLibrary.Concat_StrStr` _returnvalue "://" (`self.Host`) ":" (`KismetStringLibrary.Conv_IntToString` (`self.Port`))))))))